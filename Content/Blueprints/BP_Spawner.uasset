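; BP_Spawner is a spawner that endlessly creates actors of a configurable class at random points during play.
; On BeginPlay it gathers four scene components into an array, then spawns immediately at the world location of a random one.
; A random delay of a few seconds wires back into the spawn, forming a latent loop with no exit.
; Spawns adjust for collisions where possible but always happen.
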(event `self.ReceiveBeginPlay`
  (set `self.PointsArray` (`|MakeArray` (`self.Scene`) (`self.Scene1`) (`self.Scene2`) (`self.Scene3`)))
  (`|SpawnActorFromClass` (`self.ActorSpawnClass`) (`KismetMathLibrary.MakeTransform` (`SceneComponent.K2_GetComponentLocation` (`KismetArrayLibrary.Array_Random` (`self.PointsArray`)))) "AdjustIfPossibleButAlwaysSpawn" "OverrideRootScale" null null :!label _label)
  (`KismetSystemLibrary.Delay` (`KismetMathLibrary.RandomFloatInRange` 5.0 8.0))
  (goto _label))

(fn `UserConstructionScript`)