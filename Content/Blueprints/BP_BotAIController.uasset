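; AI controller for group bots that runs the BT_GroupBot behavior tree and raises an alarm on spotting the player.
; PawnSensing sets the IsAlarm blackboard key when it sees a player-controlled pawn.
; Sentinel set and reset functions retune walk speed, sight radius and vision angle, trading speed for sight; BeginPlay starts in the reset state.
; The AIPerception handler is disabled because its sense parameters could not be changed at runtime.
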(event `self.ReceiveBeginPlay`
  (`self.ResetSentinel`)
  (`self.RunBehaviorTree` "/Game/Blueprints/BT_GroupBot.BT_GroupBot"))

(event `self.AIPerception.OnTargetPerceptionUpdated`
  (params (Actor :type "Actor Object Reference") (Stimulus :type "AIStimulus Structure"))
  ;[1 1 1] Отключено, так как не удается изменять параметры чувств в рантайме
)

(event `self.PawnSensing.OnSeePawn`
  (params (Pawn :type "Pawn Object Reference"))
  (if (`Pawn.IsPlayerControlled` Pawn)
    (`BlackboardComponent.SetValueAsBool` (`self.Blackboard`) (`KismetStringLibrary.Conv_StringToName` "IsAlarm") true)
    (`KismetSystemLibrary.PrintString` "alarm raised")))

(fn `ResetSentinel`
  (`self.SetParams` 500.0 250.0 15.0)
  (`KismetSystemLibrary.PrintString` "sentinel resetted"))

(fn `SetParams`
  (params (MaxWalkSpeed :type "Float (double-precision)") (SightRadius :type "Float (double-precision)") (VisionAngle :type "Float (double-precision)"))
  (bind _pawnsensing (`self.PawnSensing`))
  (bind _ascharacter (cast `Character` (`self.K2_GetPawn`)))
  (set `CharacterMovementComponent.MaxWalkSpeed` MaxWalkSpeed (`Character.CharacterMovement` _ascharacter))
  (set `PawnSensingComponent.SightRadius` SightRadius _pawnsensing)
  (`PawnSensingComponent.SetPeripheralVisionAngle` _pawnsensing VisionAngle))

(fn `SetSentinel`
  (`self.SetParams` 250.0 1000.0 45.0)
  (`KismetSystemLibrary.PrintString` "sentinel setted"))

(fn `UserConstructionScript`)